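; Personaje is a character Blueprint for a partial level that moves itself continuously and changes speed while flagged as under attack.
; Tick adds Velocidad as a local offset each frame, without sweep or delta-time scaling, so movement is frame-rate dependent and ignores collision.
; A looping two-second timer runs Chequear, which compounds Velocidad by FactorMultiplcable whenever MeAtacan is true.
; VelocidadPersonaje acts as a setter for Velocidad.
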(event Custom|chequear
  (if (Variables|Propiedades|GetMeAtacan?)
    (Variables|Propiedades|SetVelocidad (* (Variables|Propiedades|GetVelocidad) (Variables|Propiedades|GetFactorMultiplcable)))))

(event EventBeginPlay
  (Utilities|Time|SetTimerbyEvent (delegate Custom|chequear) 2.0 true))

(event EventTick
  (params (DeltaSeconds :type Float%20%28single-precision%29))
  (Transformation|AddActorLocalOffset (Variables|Propiedades|GetVelocidad) false false))

(fn ConstructionScript)

(fn VelocidadPersonaje
  (params (Velocidad :type Vector))
  (Variables|Propiedades|SetVelocidad Velocidad))